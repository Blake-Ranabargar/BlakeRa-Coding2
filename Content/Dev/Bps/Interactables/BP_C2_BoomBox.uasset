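; BP_C2_BoomBox is an interactable boom box that plays music while it holds a CD.
; PlayMusic stores the CD, sets HasCD and spawns the Cat sound at the box mesh with attenuation.
; When the player character overlaps the Box with a CD loaded, it stops the sound and spawns a fresh BP_C2_CD at the Arrow.
; Without a CD, the overlap only prints "Needs CD"; AlternateUse_1 is empty.
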(event `Play Music`
  (params (CD :type "Actor Object Reference"))
  (set `self.CD` CD)
  (set `self.Has CD?` true)
  (bind _returnvalue (`GameplayStatics.SpawnSoundAtLocation` "/Game/Dev/SFXs/Cat.Cat" (`SceneComponent.K2_GetComponentLocation` (`self.SM_Box`)) (struct) 1.0 1.0 0.0 "/Game/Dev/Bps/SFXAT_C2_BoomBox.SFXAT_C2_BoomBox" null)))

(event `Alternate Use_1`)

(event `self.Box.OnComponentBeginOverlap`
  (params (OverlappedComponent :type "PrimitiveComponent Object Reference") (OtherActor :type "Actor Object Reference") (OtherComp :type "PrimitiveComponent Object Reference") (OtherBodyIndex :type Integer) (bFromSweep :type Boolean) (SweepResult :type "HitResult Structure (by ref)"))
  (cast `/Game/Dev/Bps/Character/BP_FirstPersonCharacterCustom` OtherActor)
  (if (`self.Has CD?`)
    (set `self.Has CD?` false)
    (`KismetSystemLibrary.PrintString` "CD Drop")
    (`|SpawnActorFromClass` "/Game/Dev/Bps/Interactables/BP_C2_CD.BP_C2_CD_C" (`SceneComponent.K2_GetComponentToWorld` (`self.Arrow`)) "AdjustIfPossibleButAlwaysSpawn" "MultiplyWithRoot" null null)
    (`AudioComponent.Stop` (stale `Play Music` _returnvalue))
    (else
      (`KismetSystemLibrary.PrintText` "Needs CD"))))

(fn `UserConstructionScript`)
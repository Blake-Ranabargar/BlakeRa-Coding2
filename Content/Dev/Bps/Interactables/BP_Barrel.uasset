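; BP_Barrel is an interactable storage barrel with its own inventory component and menu widget.
; A sphere overlap by the first-person character plays a timeline that rotates the lid open, and leaving reverses it.
; When opening finishes, it shows the barrel menu and player inventory and registers the inventory with GM_SaveLoad's LevelSave.
; A loadInventory event replaces the contents with saved data.
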(event `self.ReceiveBeginPlay`
  (bind _returnvalue (`|CreateWidget` "/Game/Dev/Bps/Widgets/WBP_BarrelMenu.WBP_BarrelMenu_C" null (`self.BPC_Inventory`)))
  (set `self.WBP_BarrelMenu` _returnvalue))

(event `self.Sphere_Col.OnComponentBeginOverlap`
  (params (OverlappedComponent :type "PrimitiveComponent Object Reference") (OtherActor :type "Actor Object Reference") (OtherComp :type "PrimitiveComponent Object Reference") (OtherBodyIndex :type Integer) (bFromSweep :type Boolean) (SweepResult :type "HitResult Structure (by ref)"))
  (bind _asbp_first_person_character_custom (cast `/Game/Dev/Bps/Character/BP_FirstPersonCharacterCustom` OtherActor))
  (`self.Barrel Open` false))

(event `Barrel Open`
  (params (Reverse :type Boolean))
  (if Reverse
    (bind (_direction _newtrack_0) (`Timeline|Open Timeline` :!via `Reverse` :!label _label)
      (:`Update`
        (`SceneComponent.K2_SetRelativeRotation` (`self.Barrel_Lid`) (`KismetMathLibrary.MakeRotator` (`KismetMathLibrary.Lerp` 0.0 60.0 _newtrack_0)) false false))
      (:`Finished`
        (if (not Reverse)
          (`KismetSystemLibrary.PrintText` "Open Barrel")
          (`UserWidget.AddToViewport` (`self.WBP_BarrelMenu`) 0)
          (`/Game/Dev/Bps/Character/BP_FirstPersonCharacterCustom.Show Inventory` (stale `self.Sphere_Col.OnComponentBeginOverlap` _asbp_first_person_character_custom))
          (bind _asgm_save_load (cast `/Game/Dev/Bps/Interactables/Save_Load/GM_SaveLoad` (`GameplayStatics.GetGameMode`)))
          (`/Game/Dev/Bps/Interactables/Save_Load/SG_LevelState.Add Inventory` (`/Game/Dev/Bps/Interactables/Save_Load/GM_SaveLoad.LevelSave` _asgm_save_load) (`self.BPC_Inventory`)))))
    (else
      (goto _label))))

(event `self.Sphere_Col.OnComponentEndOverlap`
  (params (OverlappedComponent :type "PrimitiveComponent Object Reference") (OtherActor :type "Actor Object Reference") (OtherComp :type "PrimitiveComponent Object Reference") (OtherBodyIndex :type Integer))
  (cast `/Game/Dev/Bps/Character/BP_FirstPersonCharacterCustom` OtherActor)
  (`self.Barrel Open` true))

(event `load Inventory`
  (params (EnumInventory :type "Array of /Game/Dev/Bps/E_Item Enum"))
  (set `/Game/Dev/Bps/Widgets/BPC_Inventory.EnumInventory` EnumInventory (`self.BPC_Inventory`)) ; Replace Current Inv with saved INV
)

(fn `UserConstructionScript`)
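; Save/load Blueprint, apparently a game mode, that persists the player and per-level state in two save slots.
; Save writes belt and inventory to SG_Player, and a location to SG_LevelState under the level name.
; Load restores inventories and transform, then calls ActivateActors on the level save.
; BeginPlay loads or creates saves, though its level check is hard-wired true; deleting the level save reopens the level.
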(event `self.ReceiveBeginPlay`
  (`KismetSystemLibrary.PrintText` "Save Load" true true (struct :`R` 1.0 :`B` 0.866449 :`A` 1.0))
  (`|ExecutionSequence`
    (:`then_0`
      (bind _returnvalue (`GameplayStatics.DoesSaveGameExist` (`self.Slot Name`)))
      (if _returnvalue
        (`self.Load`)
        (else
          (bind _returnvalue_2 (`GameplayStatics.CreateSaveGameObject` "/Game/Dev/Bps/Interactables/Save_Load/SG_Player.SG_Player_C"))
          (set `self.PlayerSave` _returnvalue_2))))
    (:`then_1`
      (bind _returnvalue_3 (`GameplayStatics.GetCurrentLevelName` true))
      (`GameplayStatics.DoesSaveGameExist` (`KismetStringLibrary.Concat_StrStr` _returnvalue_3 (`self.Slot Name`)))
      (if true
        (`self.Load`)
        (else
          (bind _returnvalue_4 (`GameplayStatics.CreateSaveGameObject` "/Game/Dev/Bps/Interactables/Save_Load/SG_LevelState.SG_LevelState_C"))
          (set `self.LevelSave` _returnvalue_4))))))

(fn `DeleteLevelSave`
  (bind _returnvalue (`GameplayStatics.GetCurrentLevelName` true))
  (`GameplayStatics.DeleteGameInSlot` _returnvalue)
  (`GameplayStatics.OpenLevel` (`KismetStringLibrary.Conv_StringToName` _returnvalue)))

(fn `DeleteSave`
  (`GameplayStatics.DeleteGameInSlot` (`self.Slot Name`))
  (`self.DeleteLevelSave`))

(fn `Load`
  (bind _playersave (`self.PlayerSave`))
  (`|ExecutionSequence`
    (:`then_0`
      (bind _returnvalue (`GameplayStatics.LoadGameFromSlot` (`self.Slot Name`))) ; Load from File
      (bind _assg_player (cast `/Game/Dev/Bps/Interactables/Save_Load/SG_Player` _returnvalue)) ; Cast to specific SG player
      (set `self.PlayerSave` _assg_player) ; Store as a variable
      (bind _asbp_first_person_character_custom (cast `/Game/Dev/Bps/Character/BP_FirstPersonCharacterCustom` (`GameplayStatics.GetPlayerCharacter` 0))) ; Get ref to player
      (`/Game/Dev/Bps/Widgets/BPC_Inventory.Set Enum Array` (`/Game/Dev/Bps/Character/BP_FirstPersonCharacterCustom.BPC_Belt_Inventory` _asbp_first_person_character_custom) (`/Game/Dev/Bps/Interactables/Save_Load/SG_Player.Belt` (`self.PlayerSave`)))
      (`/Game/Dev/Bps/Widgets/BPC_Inventory.Set Enum Array` (`/Game/Dev/Bps/Character/BP_FirstPersonCharacterCustom.BPC_Inventory` _asbp_first_person_character_custom) (`/Game/Dev/Bps/Interactables/Save_Load/SG_Player.PlayerInv` (`self.PlayerSave`)))
      (`/Game/Dev/Bps/Character/BP_FirstPersonCharacterCustom.load Transform` _asbp_first_person_character_custom (`/Game/Dev/Bps/Interactables/Save_Load/SG_Player.Location` _playersave) (`/Game/Dev/Bps/Interactables/Save_Load/SG_Player.Forward` _playersave))
      (`KismetSystemLibrary.PrintText` "Inventory Updated" true true (struct :`R` 1.0 :`B` 0.989039 :`A` 1.0)))
    (:`then_1`
      (bind _returnvalue_2 (`GameplayStatics.GetCurrentLevelName` true))
      (bind _returnvalue_3 (`GameplayStatics.LoadGameFromSlot` _returnvalue_2))
      (bind _assg_level_state (cast `/Game/Dev/Bps/Interactables/Save_Load/SG_LevelState` _returnvalue_3))
      (bind _output_get (set `self.LevelSave` _assg_level_state))
      (`/Game/Dev/Bps/Interactables/Save_Load/SG_LevelState.ActivateActors` _output_get))))

(fn `Save`
  (params (Belt :type "Array of /Game/Dev/Bps/E_Item Enum") (`Player Inv` :type "Array of /Game/Dev/Bps/E_Item Enum") (Location :type "Transform Structure") (Target :type "/Game/Dev/Bps/Interactables/Save_Load/SG_Player Object Reference") (Forward :type "Vector Structure"))
  (bind _playersave (`self.PlayerSave`))
  (bind _levelsave (`self.LevelSave`))
  (`|ExecutionSequence`
    (:`then_0`
      (set `/Game/Dev/Bps/Interactables/Save_Load/SG_Player.Belt` Belt _playersave)
      (set `/Game/Dev/Bps/Interactables/Save_Load/SG_Player.PlayerInv` `Player Inv` _playersave)
      (`GameplayStatics.SaveGameToSlot` (`self.PlayerSave`) (`self.Slot Name`)) ; Save game to file
      (`KismetSystemLibrary.PrintText` "Game saved to slot" true true (struct :`R` 0.848663 :`B` 1.0 :`A` 1.0)))
    (:`then_1`
      (set `/Game/Dev/Bps/Interactables/Save_Load/SG_LevelState.SaveLocation` Location _levelsave)
      (bind _returnvalue (`GameplayStatics.GetCurrentLevelName` true))
      (`GameplayStatics.SaveGameToSlot` _levelsave _returnvalue))))

(fn `UserConstructionScript`)
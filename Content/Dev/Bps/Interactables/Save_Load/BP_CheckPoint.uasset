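; BP_CheckPoint is a checkpoint actor that saves the game when the player walks into it.
; On BeginPlay it caches the GM_SaveLoad game mode.
; When a BP_FirstPersonCharacterCustom overlaps it, it passes the character's belt inventory, main inventory, transform and forward vector to the game mode's Save function, then prints a confirmation.
; It has no one-shot guard, so every new overlap saves again.
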(event `self.ReceiveBeginPlay`
  (bind _asgm_save_load (cast `/Game/Dev/Bps/Interactables/Save_Load/GM_SaveLoad` (`GameplayStatics.GetGameMode`)))
  (set `self.Game Mode` _asgm_save_load))

(event `self.ReceiveActorBeginOverlap`
  (params (OtherActor :type "Actor Object Reference"))
  (bind _asbp_first_person_character_custom (cast `/Game/Dev/Bps/Character/BP_FirstPersonCharacterCustom` OtherActor)) ; When Player overlaps, call save function on the gameode
  (`/Game/Dev/Bps/Interactables/Save_Load/GM_SaveLoad.Save` (`self.Game Mode`) (`/Game/Dev/Bps/Widgets/BPC_Inventory.EnumInventory` (`/Game/Dev/Bps/Character/BP_FirstPersonCharacterCustom.BPC_Belt_Inventory` _asbp_first_person_character_custom)) (`/Game/Dev/Bps/Widgets/BPC_Inventory.EnumInventory` (`/Game/Dev/Bps/Character/BP_FirstPersonCharacterCustom.BPC_Inventory` _asbp_first_person_character_custom)) (`self.GetTransform` _asbp_first_person_character_custom) null (`self.GetActorForwardVector` _asbp_first_person_character_custom))
  (`KismetSystemLibrary.PrintString` "Game saved: Checkpoint activated"))

(fn `UserConstructionScript`)
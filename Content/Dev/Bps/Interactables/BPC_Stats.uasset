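; BPC_Stats is a stats component holding a Stats struct with health, mana, stamina, experience, gold and a saved location.
; CanGetSprint reports whether stamina is above a small threshold, and Sprinting rebuilds the struct with stamina reduced by the given amount.
; A debug event prints health, mana, stamina and experience on screen, using the passed DeltaSeconds as display duration.
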(event `CustomEvent`
  (params (DeltaSeconds :type "Float (single-precision)"))
  (`self.Debgug stats` DeltaSeconds))

(event `Debgug stats`
  (params (Duration :type "Float (double-precision)"))
  (bind (_health _mana _stamina _savedlocation _gold _experience) (break `/Game/Dev/Bps/Interactables/S_Stats` (`self.Stats`)))
  (`KismetSystemLibrary.PrintText` (`|FormatText` "HP: {health}, MP: {mana}, Stam: {stamina}, XP: {experience}" _health _mana _stamina _experience) true true (make `LinearColor` 1.0 0.0 0.1) Duration))

(fn `CanGetSprint`
  (returns (`Can Sprint` :type Boolean))
  (bind (_stats_health _stats_mana _stats_stamina) (break `/Game/Dev/Bps/Interactables/S_Stats` (`self.Stats`)))
  (return (> _stats_stamina 1.0)) ; Retrun true if stamina is greater than 1
)

(fn `Sprinting`
  (params (`Reduce Stamina By` :type "Float (double-precision)"))
  (bind (_stats_health _stats_mana _stats_stamina _stats_savedlocation _stats_gold _stats_experience) (break `/Game/Dev/Bps/Interactables/S_Stats` (`self.Stats`)))
  (set `self.Stats` (make `/Game/Dev/Bps/Interactables/S_Stats` _stats_health _stats_mana (- _stats_stamina `Reduce Stamina By`) _stats_savedlocation _stats_gold _stats_experience)))
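; BP_C2_CD is a holdable CD item that can be inserted into a BP_C2_BoomBox.
; Pickup prints a message and disables box collision; Drop restores collision and physics, then applies a fixed world-X velocity impulse.
; Use line-traces forward for a boombox: an empty one starts music, destroys the CD and clears the owner's HeldItem.
; A boombox that already has a CD only gets its HasCD flag cleared.
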(event `/Game/Dev/Bps/Interactables/BPI_Item.Pickup`
  (params (Owner :type "/Game/Dev/Bps/Interactables/BPC_Interact Object Reference"))
  (`KismetSystemLibrary.PrintText` "You equiped a CD")
  (`PrimitiveComponent.SetCollisionEnabled` (`self.Box_Col`) "NoCollision"))

(event `/Game/Dev/Bps/Interactables/BPI_Item.Drop`
  (bind _box_col (`self.Box_Col`))
  (set `/Game/Dev/Bps/Interactables/BPC_Interact.HeldItem` null (stale `/Game/Dev/Bps/Interactables/BPI_Item.Pickup` Owner)) ; Set "HeldItem" to nothing
  (`PrimitiveComponent.SetCollisionEnabled` _box_col "QueryAndPhysics")
  (`PrimitiveComponent.SetSimulatePhysics` _box_col true)
  (`PrimitiveComponent.AddImpulse` _box_col (1.0 0.0 0.0) "None" true) ; Throw Item Forward
)

(event `/Game/Dev/Bps/Interactables/BPI_Item.Use`
  (bind _box_col (`self.Box_Col`))
  (bind _returnvalue (`SceneComponent.K2_GetComponentLocation` _box_col))
  (bind _outhit (`KismetSystemLibrary.LineTraceSingle` _returnvalue (+ _returnvalue (* (`SceneComponent.GetForwardVector` _box_col) 300.0)) "TraceTypeQuery1"))
  (bind _asbp_c2_boom_box (cast `/Game/Dev/Bps/Interactables/BP_C2_BoomBox` (`.HitActor` (`GameplayStatics.BreakHitResult` _outhit))))
  (if (`/Game/Dev/Bps/Interactables/BP_C2_BoomBox.Has CD?` _asbp_c2_boom_box)
    (set `/Game/Dev/Bps/Interactables/BP_C2_BoomBox.Has CD?` false _asbp_c2_boom_box)
    (else
      (set `/Game/Dev/Bps/Interactables/BP_C2_BoomBox.Has CD?` true _asbp_c2_boom_box)
      (`self.K2_DestroyActor`)
      (`/Game/Dev/Bps/Interactables/BP_C2_BoomBox.Play Music` _asbp_c2_boom_box (`/Game/Dev/Bps/Interactables/BPC_Interact.HeldItem` (stale `/Game/Dev/Bps/Interactables/BPI_Item.Pickup` Owner)))
      (set `/Game/Dev/Bps/Interactables/BPC_Interact.HeldItem` null (stale `/Game/Dev/Bps/Interactables/BPI_Item.Pickup` Owner)) ; Set "HeldItem" to nothing
    )))

(event `/Game/Dev/Bps/Interactables/BPI_Item.Alternate Use`)

(fn `UserConstructionScript`)
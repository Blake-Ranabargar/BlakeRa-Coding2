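; Pickup lighter item that can be toggled open and lit, then used to light BP_C2_Candle actors.
; Use flip-flops cap rotation timelines and the visibility of the flame and its point light, tracking a Flame flag.
; While lit, AlternateUse line traces forward from the flame, showing a hit candle's flame and light and hiding its smoke.
; Pickup disables box collision and returns the item type; Drop restores collision, enables physics and applies an impulse.
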(event `/Game/Dev/Bps/Interactables/BPI_Item.Drop`
  (bind _box_col (`self.Box_Col`))
  (`PrimitiveComponent.SetCollisionEnabled` _box_col "QueryAndPhysics")
  (`PrimitiveComponent.SetSimulatePhysics` _box_col true)
  (`PrimitiveComponent.AddImpulse` _box_col (1.0 0.0 0.0) "None" true) ; Throw Item Forward
)

(event `/Game/Dev/Bps/Interactables/BPI_Item.Use`
  (bind _lighter_flame (`self.Lighter_Flame`))
  (`/Engine/EditorBlueprintResources/StandardMacros.FlipFlop`
    (:`A`
      (`|ExecutionSequence`
        (:`then_0`
          (`Timeline|Cap_Open`
            (:`Update`
              (`SceneComponent.K2_SetRelativeRotation` :`self` (`self.Lighter_Cap`)))))
        (:`then_1`
          (`SceneComponent.SetVisibility` _lighter_flame true false)
          (`SceneComponent.SetVisibility` (`self.LighterFlame_PointLight`) true false)
          (set `self.Flame` true))))
    (:`B`
      (`|ExecutionSequence`
        (:`then_0`
          (`Timeline|Cap_Close` :!label _label
            (:`Update`
              (`SceneComponent.K2_SetRelativeRotation` (`self.Lighter_Cap`) (struct :`Pitch` -75.0) false false)
              (set `self.Flame` false))))
        (:`then_1`
          (goto _label :!via `Reverse`))
        (:`then_2`
          (`SceneComponent.SetVisibility` _lighter_flame false false)
          (`SceneComponent.SetVisibility` (`self.LighterFlame_PointLight`) false false))))))

(event `/Game/Dev/Bps/Interactables/BPI_Item.Alternate Use`
  (bind _lighter_flame (`self.Lighter_Flame`))
  (bind _returnvalue (`SceneComponent.K2_GetComponentLocation` _lighter_flame))
  (if (`self.Flame`)
    (bind _outhit (`KismetSystemLibrary.LineTraceSingle` :`Start` _returnvalue :`End` (+ _returnvalue (* (`SceneComponent.GetForwardVector` _lighter_flame) 300.0)) :`TraceChannel` "TraceTypeQuery1" :`DrawDebugType` "ForDuration"))
    (`|ExecutionSequence`
      (:`then_0`
        (bind (_bblockinghit _binitialoverlap _time _distance _location _impactpoint _normal _impactnormal _physmat _hitactor) (`GameplayStatics.BreakHitResult` _outhit))
        (bind _asbp_c2_candle (cast `/Game/Dev/Bps/Interactables/BP_C2_Candle` _hitactor))
        (`SceneComponent.SetVisibility` (`/Game/Dev/Bps/Interactables/BP_C2_Candle.NE_Flame` _asbp_c2_candle) true false)
        (`SceneComponent.SetVisibility` (`/Game/Dev/Bps/Interactables/BP_C2_Candle.Flame_PointLight` _asbp_c2_candle) true false)
        (`KismetSystemLibrary.PrintText` "Candle Lights on"))
      (:`then_1`
        (bind _asbp_c2_candle_2 (cast `/Game/Dev/Bps/Interactables/BP_C2_Candle` _hitactor))
        (`SceneComponent.SetVisibility` (`/Game/Dev/Bps/Interactables/BP_C2_Candle.NE_Smoke` _asbp_c2_candle_2) false false)
        (`KismetSystemLibrary.PrintText` "Hello")))
    (else
      (`KismetSystemLibrary.PrintText` "Light not on"))))

(fn `Pickup`
  (params (Owner :type "/Game/Dev/Bps/Interactables/BPC_Interact Object Reference"))
  (returns (ItemType :type "/Game/Dev/Bps/E_Item Enum"))
  (`KismetSystemLibrary.PrintText` "You equiped a Lighter")
  (`PrimitiveComponent.SetCollisionEnabled` (`self.Box_Col`) "NoCollision")
  (return (`self.Item Type`)))

(fn `UserConstructionScript`)
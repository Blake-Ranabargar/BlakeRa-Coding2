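; Interactable door Blueprint that stays locked until PickupKey sets HasKey.
; With the key, Interact flip-flops a timeline that swings the mesh yaw open or shut, with a one-time opening sound; without it, a locked sound plays.
; Separately, Activate calls OpenDoor, which adds the door to the GM_SaveLoad game mode's LevelSave and destroys the actor.
; Both sounds play at world origin rather than the door's location.
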(event `self.Interact`
  (if (`self.Has Key?`)
    (`/Engine/EditorBlueprintResources/StandardMacros.FlipFlop`
      (:`A`
        (bind (_direction _door_track) (`Timeline|Door Timeline` :!label _label)
          (:`Update`
            (`SceneComponent.K2_SetRelativeRotation` (`self.SM_Door`) (`KismetMathLibrary.MakeRotator` 0.0 0.0 (`KismetMathLibrary.Lerp` 0.0 110.0 _door_track)) false false)
            (`/Engine/EditorBlueprintResources/StandardMacros.DoOnce` false
              (:`Completed`
                (`GameplayStatics.PlaySoundAtLocation` "/Game/Dev/SFXs/OpenDoor_SFX.OpenDoor_SFX" (0.0 0.0 0.0) (struct) 1.0 1.0 0.0 null null null null))))))
      (:`B`
        (goto _label :!via `Reverse`)))
    (else
      (`GameplayStatics.PlaySoundAtLocation` "/Game/Dev/SFXs/LockedDoor_SFX.LockedDoor_SFX" (0.0 0.0 0.0) (struct) 1.0 1.0 0.0 null null null null))))

(event `self.Pickup_Key`
  (set `self.Has Key?` true))

(event `/Game/Dev/Bps/BPI_Activatable.Activate`
  (`self.Open Door`))

(event `Open Door`
  (bind _asgm_save_load (cast `/Game/Dev/Bps/Interactables/Save_Load/GM_SaveLoad` (`GameplayStatics.GetGameMode`)))
  (`/Game/Dev/Bps/Interactables/Save_Load/SG_LevelState.AddActor` (`/Game/Dev/Bps/Interactables/Save_Load/GM_SaveLoad.LevelSave` _asgm_save_load) self)
  (`self.K2_DestroyActor`))

(fn `UserConstructionScript`)
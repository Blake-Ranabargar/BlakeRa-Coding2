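; BP_C2_Key is a key interactable that the player picks up, drops or uses to remove a door.
; Pickup prints a message and disables box collision; dropping clears the owner's HeldItem, restores collision and physics, and applies a fixed world-X impulse.
; Use traces forward from the box and, on hitting a BP_C2_Door, clears HeldItem and destroys the door.
; A Pickup function returns an enum value, and AlternateUse is empty.
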(event `Pickup_key`
  (params (Owner :type "/Game/Dev/Bps/Interactables/BPC_Interact Object Reference"))
  (`KismetSystemLibrary.PrintText` "You found a key!")
  (`PrimitiveComponent.SetCollisionEnabled` (`self.Box_Col`) "NoCollision"))

(event `/Game/Dev/Bps/Interactables/BPI_Item.Drop`
  (bind _box_col (`self.Box_Col`))
  (set `/Game/Dev/Bps/Interactables/BPC_Interact.HeldItem` null (stale `Pickup_key` Owner)) ; Set "HeldItem" to nothing
  (`PrimitiveComponent.SetCollisionEnabled` _box_col "QueryAndPhysics")
  (`PrimitiveComponent.SetSimulatePhysics` _box_col true)
  (`PrimitiveComponent.AddImpulse` _box_col (1.0 0.0 0.0) "None" true) ; Throw Item Forward
)

(event `/Game/Dev/Bps/Interactables/BPI_Item.Use`
  (bind _box_col (`self.Box_Col`))
  (bind _returnvalue (`SceneComponent.K2_GetComponentLocation` _box_col))
  (bind _outhit (`KismetSystemLibrary.LineTraceSingle` _returnvalue (+ _returnvalue (* (`SceneComponent.GetForwardVector` _box_col) 300.0)) "TraceTypeQuery1"))
  (bind _asbp_c2_door (cast `/Game/Dev/Bps/Interactables/BP_C2_Door` (`.HitActor` (`GameplayStatics.BreakHitResult` _outhit))))
  (set `/Game/Dev/Bps/Interactables/BPC_Interact.HeldItem` null (stale `Pickup_key` Owner)) ; Set "HeldItem" to nothing
  (`self.K2_DestroyActor` _asbp_c2_door))

(event `/Game/Dev/Bps/Interactables/BPI_Item.Alternate Use`)

(fn `Pickup`
  (params (Owner :type "/Game/Dev/Bps/Interactables/BPC_Interact Object Reference"))
  (returns (ItemType :type "/Game/Dev/Bps/E_Item Enum"))
  (return "NewEnumerator3"))

(fn `UserConstructionScript`)
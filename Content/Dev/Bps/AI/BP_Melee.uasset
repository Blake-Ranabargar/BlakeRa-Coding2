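; BP_Melee is a melee AI actor that tracks its own health and dies when it runs out.
; Taking damage reports an AI damage sense event at the instigator pawn's location, then subtracts from Health, destroying the actor at zero or below as a placeholder for a later ragdoll.
; A GetMedkit event adds health, clamped to a normalized zero-to-one range.
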(event `self.ReceiveAnyDamage`
  (params (Damage :type "Float (single-precision)") (DamageType :type "DamageType Object Reference") (InstigatedBy :type "Controller Object Reference") (DamageCauser :type "Actor Object Reference"))
  (`AISense_Damage.ReportDamageEvent` null InstigatedBy Damage (`self.K2_GetActorLocation` (`Controller.K2_GetPawn` InstigatedBy)))
  (bind _output_get (set `self.Health` (- (`self.Health`) Damage)))
  (if (not (> _output_get 0.0))
    (`KismetSystemLibrary.PrintText` "We are dead")
    (`self.K2_DestroyActor`) ; Change to ragdoll later
  ))

(event `Get Medkit`
  (params (`Helth to Add` :type "Float (double-precision)"))
  (set `self.Health` (`KismetMathLibrary.FClamp` (+ (`self.Health`) `Helth to Add`))))

(fn `UserConstructionScript`)
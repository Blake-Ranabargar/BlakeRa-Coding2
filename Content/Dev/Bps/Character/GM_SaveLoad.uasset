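; Save/load manager actor that persists the player's belt and main inventory to a save slot.
; On BeginPlay it loads the existing slot after a short delay, or creates a new SG_Player save object if none exists.
; Save copies both inventory arrays into that object and writes it to the slot.
; Load pushes the stored arrays into the inventory components on BP_FirstPersonCharacterCustom.
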(event `self.ReceiveBeginPlay`
  (`KismetSystemLibrary.PrintText` "Save Load" true true (struct :`R` 1.0 :`B` 0.866449 :`A` 1.0))
  (`GameplayStatics.DoesSaveGameExist` (`self.Slot Name`))
  (if true
    (`KismetSystemLibrary.Delay` 0.2)
    (`self.Load`)
    (else
      (bind _returnvalue (`GameplayStatics.CreateSaveGameObject` "/Game/Dev/Bps/Interactables/SG_Player.SG_Player_C"))
      (set `self.PlayerSave` _returnvalue))))

(fn `Load`
  (bind _returnvalue (`GameplayStatics.LoadGameFromSlot` (`self.Slot Name`))) ; Load from File
  (bind _assg_player (cast `/Game/Dev/Bps/Interactables/SG_Player` _returnvalue)) ; Cast to specific SG player
  (set `self.PlayerSave` _assg_player) ; Store as a variable
  (bind _asbp_first_person_character_custom (cast `/Game/Dev/Bps/Character/BP_FirstPersonCharacterCustom` (`GameplayStatics.GetPlayerCharacter` 0))) ; Get ref to player
  (`/Game/Dev/Bps/Widgets/BPC_Inventory.Set Enum Array` (`/Game/Dev/Bps/Character/BP_FirstPersonCharacterCustom.BPC_Belt_Inventory` _asbp_first_person_character_custom) (`/Game/Dev/Bps/Interactables/SG_Player.Belt` (`self.PlayerSave`)))
  (`/Game/Dev/Bps/Widgets/BPC_Inventory.Set Enum Array` (`/Game/Dev/Bps/Character/BP_FirstPersonCharacterCustom.BPC_Inventory` _asbp_first_person_character_custom) (`/Game/Dev/Bps/Interactables/SG_Player.PlayerInv` (`self.PlayerSave`)))
  (`KismetSystemLibrary.PrintText` "Inventory Updated" true true (struct :`R` 1.0 :`B` 0.989039 :`A` 1.0)))

(fn `Save`
  (params (Belt :type "Array of /Game/Dev/Bps/E_Item Enum") (`Player Inv` :type "Array of /Game/Dev/Bps/E_Item Enum"))
  (bind _playersave (`self.PlayerSave`))
  (set `/Game/Dev/Bps/Interactables/SG_Player.Belt` Belt _playersave)
  (set `/Game/Dev/Bps/Interactables/SG_Player.PlayerInv` `Player Inv` _playersave)
  (`GameplayStatics.SaveGameToSlot` (`self.PlayerSave`) (`self.Slot Name`)) ; Save game to file
  (`KismetSystemLibrary.PrintText` "Game saved to slot" true true (struct :`R` 0.848663 :`B` 1.0 :`A` 1.0)))

(fn `UserConstructionScript`)